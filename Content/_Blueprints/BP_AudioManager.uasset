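; Audio manager actor that plays fountain sounds in response to force updates from IfMagicNexus.
; On each update it prints the Strength, then calls StartAudio when it reaches a fixed threshold, otherwise StopAudio.
; StartAudio attaches the intro cue and binds its finish event, with OnSoundStopped spawning the middle cue.
; StopAudio destroys the stored component, if valid, and spawns the end cue.
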(event Custom|OnSoundStopped
  (bind _returnvalue (Audio|SpawnSoundAttached "/Game/Audio/SC_FountainMiddle.SC_FountainMiddle" (Variables|Default|GetDefaultSceneRoot) "None" "0, 0, 0" "0, 0, 0" "KeepRelativeOffset" false 1.0 1.0 0.0 0 0))
  (Variables|Default|SetAudioComponent _returnvalue))

(event Custom|On%20Force%20Updated
  (params (Raw :type Integer) (Strength :type Integer))
  (Development|PrintString (Utilities|String|ToString(Integer) Strength))
  (if (>= Strength 20)
    (CallFunction|StartAudio)
    (else
      (CallFunction|StopAudio))))

(event EventBeginPlay
  (EventDispatchers|BindEventtoOnForceUpdated (Variables|Default|GetIfMagicNexus) (EventDispatchers|CreateEvent :!event Custom|On%20Force%20Updated)))

(fn ConstructionScript)

(fn StopAudio
  (Utilities|IsValid (Variables|Default|GetAudioComponent)
    (:Is%20Valid
      ;[1 1 1] Destroys old component and plays the end sound
      (Components|DestroyComponent (Variables|Default|GetAudioComponent))
      (bind _returnvalue (Audio|SpawnSoundAttached "/Game/Audio/SC_FountainEnd.SC_FountainEnd" (Variables|Default|GetDefaultSceneRoot) "None" "0, 0, 0" "0, 0, 0" "KeepRelativeOffset" false 1.0 1.0 0.0 0 0))
      (Variables|Default|SetAudioComponent _returnvalue))))

(fn StartAudio
  ;[1 1 1] Destroy it audio was previously played
  (Utilities|IsValid (Variables|Default|GetAudioComponent)
    (:Is%20Valid
      (Components|DestroyComponent (Variables|Default|GetAudioComponent)))
    (:Is%20Not%20Valid
      _))
  ;[1 1 1] Attach audio component to this actor
  (bind _returnvalue (Audio|SpawnSoundAttached "/Game/Audio/SC_Fountain.SC_Fountain" (Variables|Default|GetDefaultSceneRoot) "None" "0, 0, 0" "0, 0, 0" "KeepRelativeOffset" false 1.0 1.0 0.0 0 0))
  (EventDispatchers|BindEventtoOnAudioFinished _returnvalue (EventDispatchers|CreateEvent :!event Custom|OnSoundStopped)))